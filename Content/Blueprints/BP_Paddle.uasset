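; BP_Paddle is a player-controlled paddle that moves sideways with swept movement through Enhanced Input and forwards the action press to BP_GameManager.
; BeginPlay registers the input mapping context and caches the game manager.
; GetTopNormal fakes a curved top surface by rotating the hit normal in proportion to its offset from center, up to a maximum tilt.
; Tick draws debug arrows previewing these normals across the top.
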(event Input|EnhancedActionEvents|EnhancedInputActionIA_Move
  (params (ActionValue :type Float%20%28double-precision%29) (ElapsedSeconds :type Float%20%28double-precision%29) (TriggeredSeconds :type Float%20%28double-precision%29) (InputAction :type Input%20Action%20Object%20Reference :default "/Game/IA_Move.IA_Move"))
  (Transformation|SetActorLocation (+ (* (* (* (Class|KismetMathLibrary|VectorRight) ActionValue) (Variables|コンポーネント|GetSpeed)) (Utilities|Time|GetWorldDeltaSeconds)) (Transformation|GetActorLocation)) true false))

(event Input|EnhancedActionEvents|EnhancedInputActionIA_Action
  (params (ActionValue :type Boolean) (ElapsedSeconds :type Float%20%28double-precision%29) (TriggeredSeconds :type Float%20%28double-precision%29) (InputAction :type Input%20Action%20Object%20Reference :default "/Game/IA_Action.IA_Action"))
  (:Started
    (Default|Action (Variables|Default|GetGameManager))))

(event EventBeginPlay
  (Input|AddMappingContext (PlayerController|LocalPlayerSubsystems|GetEnhancedInputLocalPlayerSubsystem (Game|GetPlayerController 0)) "/Game/IMC_InGame.IMC_InGame" 0 "(bIgnoreAllPressedKeysUntilRelease=True,bForceImmediately=False,bNotifyUserSettings=False)")
  (bind _returnvalue (Actor|GetActorOfClass "/Game/Blueprints/BP_GameManager.BP_GameManager_C"))
  (Variables|Default|SetGameManager _returnvalue))

(event Collision|EventActorBeginOverlap
  (params (OtherActor :type Actor%20Object%20Reference)))

(event EventTick
  (params (DeltaSeconds :type Float%20%28single-precision%29))
  (CallFunction|DrawDebugTopSurfaceNormals))

(fn ConstructionScript)

(fn GetTopNormal
  (params (HitLocation :type Vector) (Normal :type Vector))
  (bind (_origin _boxextent) (Collision|GetActorBounds false false))
  (if (Class|KismetMathLibrary|NotEqualExactlyVectorVector Normal (Math|Vector|VectorUp))
    (return true (Math|Vector|RotateVector Normal (Math|Rotator|MakeRotator (* (/ (- (.Y (Math|Vector|BreakVector HitLocation)) (.y _origin)) (.y _boxextent)) (Variables|Default|GetmaxTiltNormalDeg)) 0.0 0.0)))))

(fn DrawDebugArrow
  (params (Origin :type Vector) (Direction :type Vector))
  (bind _output_get (Variables|Default|SetL_ShapedDirection (* (Math|Vector|Normalize Direction) (Variables|Default|GetL_Length))))
  (Rendering|Debug|DrawDebugArrow Origin (+ Origin _output_get) 1e+02 "(R=0.000000,G=0.348504,B=1.000000,A=1.000000)" 0.0 1e+01 "Foreground"))

(fn DrawDebugTopSurfaceNormals
  (bind (_origin _boxextent) (Collision|GetActorBounds false false))
  (for _index (range (* (Variables|Default|GetL_DrawNumHalf) -1) (Variables|Default|GetL_DrawNumHalf))
    (bind _outnormal (CallFunction|GetTopNormal (+ (Math|Vector|MakeVector 0.0 (* (/ (.y _boxextent) (Variables|Default|GetL_DrawNumHalf)) _index) (.z _boxextent)) _origin) (Math|Vector|VectorUp)))
    (CallFunction|DrawDebugArrow (+ (Math|Vector|MakeVector 0.0 (* (/ (.y _boxextent) (Variables|Default|GetL_DrawNumHalf)) _index) (.z _boxextent)) _origin) _outnormal)))